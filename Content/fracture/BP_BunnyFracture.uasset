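; BP_BunnyFracture rebuilds a bunny static mesh as a procedural mesh at runtime, apparently as groundwork for fracturing.
; On BeginPlay it reads vertices and triangles from LOD 0, section 0 of Original_bunny, then creates a ProceduralMesh section from them, without passing normals or UVs.
; Polygon creation, mesh slicing and construction-script extraction nodes are unconnected, so no fracture occurs yet.
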(event `self.ReceiveBeginPlay`
  (`|ExecutionSequence`
    (:`then_0`
      (bind (_vertices _triangles) (`KismetProceduralMeshLibrary.GetSectionFromStaticMesh` "/Game/models/original_bunny.original_bunny"))
      (set `self.OriginVertex` _vertices)
      (set `self.OriginFace` _triangles))
    (:`then_1`
      (`ProceduralMeshComponent.CreateMeshSection_LinearColor` :`self` (`self.ProceduralMesh`) :`Vertices` (`self.OriginVertex`) :`Triangles` (`self.OriginFace`)))))

(fn `UserConstructionScript`)